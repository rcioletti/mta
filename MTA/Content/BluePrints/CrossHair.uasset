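; HUD Blueprint that draws a dynamic four-line crosshair with a small center marker at screen middle.
; Each frame DrawHUD offsets four white rectangles by AccuracyModifier plus the player character's speed-based spread, which is scaled down and capped.
; CrossHairLineLength sets arm length, and drawing runs only when HideHUD is true, despite the variable's name.
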(event `self.ReceiveDrawHUD`
  (params (SizeX :type Integer) (SizeY :type Integer))
  (bind _linearcolor (make `LinearColor` 1.0 1.0 1.0 1.0))
  (bind _crosshairlinelength (`self.CrossHairLineLength`))
  (bind _returnvalue (`KismetMathLibrary.Conv_IntToDouble` (/ SizeY 2)))
  (bind _returnvalue_2 (`KismetMathLibrary.Conv_IntToDouble` (/ SizeX 2)))
  (bind _returnvalue_3 (+ (`self.AccuracyModifier`) (`KismetMathLibrary.FMin` (/ (`KismetMathLibrary.VSize` (`self.GetVelocity` (`GameplayStatics.GetPlayerCharacter` 0))) 8.0) 40.0)))
  (if (`self.HideHUD`)
    (`|ExecutionSequence`
      (:`then_0`
        (`self.DrawRect` _linearcolor (- (- _returnvalue_2 _returnvalue_3) _crosshairlinelength) _returnvalue _crosshairlinelength 3.0)
        (`self.DrawRect` _linearcolor (+ _returnvalue_3 _returnvalue_2 0.0) _returnvalue _crosshairlinelength 3.0)
        (`self.DrawRect` _linearcolor _returnvalue_2 (- (- _returnvalue _returnvalue_3) _crosshairlinelength) 3.0 _crosshairlinelength)
        (`self.DrawRect` _linearcolor _returnvalue_2 (+ _returnvalue_3 _returnvalue) 3.0 _crosshairlinelength))
      (:`then_1`
        (`self.DrawTexture` null _returnvalue_2 _returnvalue 4.0 4.0 0.0 0.0 0.0 0.0 _linearcolor)))))

(fn `UserConstructionScript`)